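; Tower defence turret that picks a pawn within its sensing range and rotates its cannon toward it.
; Every tick, a sphere overlap gathers pawns, with distance and line-of-sight checks meant to select the closest visible one.
; The loop overwrites the best target with each element and never sets the current-target variable it traces to, so that selection is flawed.
; The cannon turns at constant speed; no firing logic exists.
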(event EventTick
  (params (DeltaSeconds :type Float%20%28single-precision%29))
  (Private|FindBestTarget)
  (Variables|Private|GetTarget
    (:then
      (Private|UpdateTurretRotation DeltaSeconds))
    (:else)))

(fn ConstructionScript)

(fn FindBestTarget
  (LocalVariables|SetBestDistance%20%28local%29 (stale _result))
  (bind _outactors (Collision|SphereOverlapActors (Transformation|GetActorLocation) (Variables|Constants|GetSensingRange) (Utilities|Array|MakeArray "ObjectTypeQuery3") "/Script/Engine.Actor"))
  (for _array_element _outactors
    (bind _output_get (LocalVariables|SetBestTarget%20%28local%29 _array_element))
    (bind _output_get_2 (LocalVariables|SetCurrentDistance%20%28local%29 (Transformation|GetDistanceTo _output_get self)))
    (if (or (< _output_get_2 (LocalVariables|GetBestDistance%20%28local%29)) (not (Utilities|IsValid (LocalVariables|GetBestTarget%20%28local%29)))) ; is this the closest target so far
      (bind _result (CallFunction|HasLineOfSight (Transformation|GetWorldLocation (Variables|Default|GetSM_Cannon)) (Transformation|GetActorLocation (LocalVariables|GetCurrentTarget%20%28local%29)) (Utilities|Array|MakeArray self (LocalVariables|GetCurrentTarget%20%28local%29))))
      (if _result
        (LocalVariables|SetBestTarget%20%28local%29 (LocalVariables|GetCurrentTarget%20%28local%29))
        (LocalVariables|SetBestDistance%20%28local%29 (LocalVariables|GetCurrentDistance%20%28local%29)))))
  (Variables|Private|SetTarget (LocalVariables|GetBestTarget%20%28local%29)))

(fn UpdateTurretRotation
  (params (DeltaSeconds :type Float%20%28double-precision%29))
  (Transformation|SetWorldRotation (Variables|Default|GetSM_Cannon) (Class|KismetMathLibrary|RInterptoConstant (Transformation|GetWorldRotation (Variables|Default|GetSM_Cannon)) (Math|Rotator|FindLookatRotation (Transformation|GetWorldLocation (Variables|Default|GetSM_Cannon)) (Transformation|GetActorLocation (Variables|Private|GetTarget))) DeltaSeconds (Variables|Constants|GetRotationSpeed)) false false))