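; Radial lightning VFX actor that fans out a set of beam particle emitters around its location.
; On BeginPlay it spawns BeamCount copies of the DistanceBeamSource emitter at the root, stepping yaw by DistributionAngle divided by BeamCount.
; The spawned components are stored in BeamArray and destroyed with the actor; that cleanup loop runs one index past BeamCount.
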(event EventBeginPlay
  (bind _beamcount (Variables|Default|GetBeamCount))
  (for _index (range 0 (- _beamcount 1))
    (bind _returnvalue (Effects|SpawnEmitteratLocation (Variables|Default|GetDistanceBeamSource) (Transformation|GetWorldLocation (Variables|Default|GetDefaultSceneRoot)) (Variables|Default|GetBeamRotator)))
    (Utilities|Array|Add (Variables|Default|GetBeamArray) _returnvalue)
    (Variables|Default|SetBeamRotator (Math|Rotator|MakeRotator (.Roll (Math|Rotator|BreakRotator (Variables|Default|GetBeamRotator))) (.Pitch (Math|Rotator|BreakRotator (Variables|Default|GetBeamRotator))) (+ (.Yaw (Math|Rotator|BreakRotator (Variables|Default|GetBeamRotator))) (/ (Variables|Default|GetDistributionAngle) (Math|Conversions|ToFloat(Integer) _beamcount)))))))

(event Collision|EventActorBeginOverlap
  (params (OtherActor :type Actor%20Object%20Reference)))

(event EventDestroyed
  (for _index (range 0 (Variables|Default|GetBeamCount))
    (Components|DestroyComponent (Utilities|Array|Get(acopy) (Variables|Default|GetBeamArray) _index))))

(event EventTick
  (params (DeltaSeconds :type Float%20%28single-precision%29)))

(fn ConstructionScript)