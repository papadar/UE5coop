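; Beam VFX actor that fires a particle beam along its forward vector to the first traced hit.
; BeginPlay traces once, spawning beam, impact emitter, randomized tinted decal and an extra effect for Pawn hits.
; Tick updates beam endpoints and emitters: CenterObject tracks the hit actor's XY at hit height; otherwise the offset math cancels to the original hit point, though the Pawn effect still centers.
; Destroyed removes spawned components.
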(event EventBeginPlay
  (bind _returnvalue (Transformation|GetActorLocation))
  (bind _defaultsceneroot (Variables|Default|GetDefaultSceneRoot))
  (bind _returnvalue_2 (Math|Vector|GetForwardVector _defaultsceneroot))
  (bind _returnvalue_3 (Effects|SpawnEmitteratLocation (Variables|Default|GetBeamSource) _returnvalue (Math|Conversions|RotationFromXVector _returnvalue_2) "1.000000,1.000000,1.000000" false))
  (bind _output_get (Variables|Default|SetBeamObject _returnvalue_3))
  (Class|ParticleSystemComponent|SetBeamSourcePoint _output_get 0 _returnvalue)
  (bind _outhit (Collision|LineTraceByChannel _returnvalue (+ _returnvalue (* _returnvalue_2 (Variables|Default|GetDistance))) "TraceTypeQuery1" false 0 "None"))
  (Variables|Components|SetHitActor (.HitActor (Collision|BreakHitResult _outhit)))
  (Variables|Components|SetHItLoc (.Location (Collision|BreakHitResult _outhit)))
  (Variables|Default|SetHitNormal (.Normal (Collision|BreakHitResult _outhit)))
  (bind _returnvalue_4 (Rendering|Material|CreateDynamicMaterialInstance (Variables|Default|GetHItDecal) "None" "None" :!class /Script/Engine.KismetMaterialLibrary))
  (Rendering|Material|SetVectorParameterValue _returnvalue_4 "Color" (Variables|Default|GetDecalColor) :!class /Script/Engine.MaterialInstanceDynamic)
  (Rendering|Material|SetScalarParameterValue _returnvalue_4 "Frame" (Math|Conversions|ToFloat(Integer) (Math|Random|RandomInteger 3)) :!class /Script/Engine.MaterialInstanceDynamic)
  (if (Variables|Default|GetCenterObject)
    (Variables|Default|SetTempSpawnLoc (Math|Vector|MakeVector (.X (Math|Vector|BreakVector (Transformation|GetActorLocation (Variables|Components|GetHitActor)))) (.Y (Math|Vector|BreakVector (Transformation|GetActorLocation (Variables|Components|GetHitActor)))) (+ (- (.Z (Math|Vector|BreakVector (Variables|Components|GetHItLoc))) (.Z (Math|Vector|BreakVector (Transformation|GetActorLocation (Variables|Components|GetHitActor))))) (.Z (Math|Vector|BreakVector (Transformation|GetActorLocation (Variables|Components|GetHitActor)))))))
    (else
      (Variables|Default|SetTempSpawnLoc (Math|Vector|MakeVector (+ (- (.X (Math|Vector|BreakVector (Variables|Components|GetHItLoc))) (.X (Math|Vector|BreakVector (Transformation|GetActorLocation (Variables|Components|GetHitActor))))) (.X (Math|Vector|BreakVector (Transformation|GetActorLocation (Variables|Components|GetHitActor))))) (+ (- (.Y (Math|Vector|BreakVector (Variables|Components|GetHItLoc))) (.Y (Math|Vector|BreakVector (Transformation|GetActorLocation (Variables|Components|GetHitActor))))) (.Y (Math|Vector|BreakVector (Transformation|GetActorLocation (Variables|Components|GetHitActor))))) (+ (- (.Z (Math|Vector|BreakVector (Variables|Components|GetHItLoc))) (.Z (Math|Vector|BreakVector (Transformation|GetActorLocation (Variables|Components|GetHitActor))))) (.Z (Math|Vector|BreakVector (Transformation|GetActorLocation (Variables|Components|GetHitActor)))))))))
  (bind _returnvalue_5 (Effects|SpawnEmitteratLocation (Variables|Default|GetCollisionEmitter) (Variables|Default|GetTempSpawnLoc) (Math|Conversions|RotationFromXVector (.Normal (Collision|BreakHitResult _outhit))) "1.000000,1.000000,1.000000" false))
  (Variables|Default|SetCollisionEmitterTemp _returnvalue_5)
  (bind _returnvalue_6 (Rendering|Decal|SpawnDecalatLocation _returnvalue_4 (Math|Conversions|ToVector(Float) (Math|Random|RandomFloatinRange 1e+02 1.5e+02)) (Variables|Default|GetTempSpawnLoc) (Math|Conversions|RotationFromXVector (.Normal (Collision|BreakHitResult _outhit))) 0.0))
  (Variables|Default|SetDecalTemp _returnvalue_6)
  (Utilities|Casting|CastToPawn (Variables|Components|GetHitActor))
  (bind _returnvalue_7 (Effects|SpawnEmitteratLocation (Variables|Default|GetTargetPawnEffect) (Variables|Default|GetTempSpawnLoc) (Math|Conversions|RotationFromXVector (.Normal (Collision|BreakHitResult _outhit))) "1.000000,1.000000,1.000000" false))
  (Variables|Default|SetTargetPawnEffectTemp _returnvalue_7))

(event Collision|EventActorBeginOverlap
  (params (OtherActor :type Actor%20Object%20Reference)))

(event EventDestroyed
  (bind _decaltemp (Variables|Default|GetDecalTemp))
  (Components|DestroyComponent (Variables|Default|GetBeamObject))
  (Components|DestroyComponent (Variables|Default|GetCollisionEmitterTemp))
  (Components|DestroyComponent (Variables|Default|GetTargetPawnEffectTemp))
  (if (not (== _decaltemp 0))
    (Components|DestroyComponent _decaltemp)))

(event EventTick
  (params (DeltaSeconds :type Float%20%28single-precision%29))
  (bind _returnvalue (Transformation|GetActorLocation))
  (bind _emmiterindex (Variables|Default|GetEmmiterIndex))
  (bind _hitloc (Variables|Components|GetHItLoc))
  (bind _hitactor (Variables|Components|GetHitActor))
  (bind _beamobject (Variables|Default|GetBeamObject))
  (bind _collisionemittertemp (Variables|Default|GetCollisionEmitterTemp))
  (bind _targetpawneffecttemp (Variables|Default|GetTargetPawnEffectTemp))
  (bind _hitloc_2 (Variables|Components|GetHItLoc))
  (bind _z (Math|Vector|BreakVector _hitloc_2))
  (bind _returnvalue_2 (Transformation|GetActorLocation _hitactor))
  (bind _returnvalue_3 (== _targetpawneffecttemp 0))
  (bind (_x _y _z_2) (Math|Vector|BreakVector _hitloc))
  (bind _returnvalue_4 (== _collisionemittertemp 0))
  (bind (_x_2 _y_2 _z_3) (Math|Vector|BreakVector _returnvalue_2))
  (bind (_x_3 _y_3 _z_4) (Math|Vector|BreakVector _returnvalue_2))
  (bind _returnvalue_5 (- _z _z_3))
  (bind _returnvalue_6 (- _y _y_3))
  (bind _returnvalue_7 (- _x _x_3))
  (bind _returnvalue_8 (- _z_2 _z_4))
  (bind _returnvalue_9 (+ _returnvalue_5 _z_3))
  (bind _returnvalue_10 (+ _returnvalue_6 _y_3))
  (bind _returnvalue_11 (+ _returnvalue_7 _x_3))
  (bind _returnvalue_12 (+ _returnvalue_8 _z_4))
  (bind _returnvalue_13 (Math|Vector|MakeVector _x_2 _y_2 _returnvalue_9))
  (bind _returnvalue_14 (Math|Vector|MakeVector _returnvalue_11 _returnvalue_10 _returnvalue_12))
  ;[1 1 1] UpdateTargetPoint
  (if (not (== _hitactor 0))
    (if (Variables|Default|GetCenterObject)
      ;;[1 1 1] Center XY, on actor
      (Class|ParticleSystemComponent|SetBeamTargetPoint _beamobject _emmiterindex _returnvalue_13)
      (Class|ParticleSystemComponent|SetBeamSourcePoint _beamobject _emmiterindex _returnvalue)
      (if (not _returnvalue_4)
        (Transformation|SetWorldLocation _collisionemittertemp _returnvalue_13 false true)
        (if (not _returnvalue_3)
          (Transformation|SetWorldLocation _targetpawneffecttemp _returnvalue_13 false true)))
      (else
        ;;[1 1 1] Stick Hit Point to actor
        (Class|ParticleSystemComponent|SetBeamTargetPoint _beamobject _emmiterindex _returnvalue_14)
        (Class|ParticleSystemComponent|SetBeamSourcePoint _beamobject _emmiterindex _returnvalue)
        (if (not _returnvalue_4)
          (Transformation|SetWorldLocation _collisionemittertemp _returnvalue_14 false true)
          (if (not _returnvalue_3)
            (Transformation|SetWorldLocation _targetpawneffecttemp _returnvalue_13 false true)))))))

(fn ConstructionScript)